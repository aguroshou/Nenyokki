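; BP_PlayerRoot is a player actor that steers toward the mouse cursor and moves continuously.
; Each tick it sets its pitch from a look-at toward Destination with a fixed offset, then refreshes Destination from a cursor Visibility trace, printing the hit.
; It then advances along its up vector by a fixed per-frame step, without delta time or sweep.
; Disconnected movement, interpolation and plane-intersection experiments remain unused.
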(event EventBeginPlay
  (Variables|Default|SetTarget 0))

(event Collision|EventActorBeginOverlap
  (params (OtherActor :type Actor%20Object%20Reference)))

(event EventTick
  (params (DeltaSeconds :type Float%20%28single-precision%29))
  (bind _returnvalue (Game|GetPlayerController 0))
  (bind (_worldlocation _worlddirection) (Game|Player|ConvertMouseLocationToWorldSpace _returnvalue))
  (Utilities|FlowControl|Sequence
    (:then_0
      (Transformation|SetActorRotation (Math|Rotator|MakeRotator 0.0 (+ (.pitch (Math|Rotator|FindLookatRotation (Transformation|GetActorLocation) (Variables|Default|GetDestination))) -8e+01) 0.0)))
    (:then_1
      (bind _outhit (Collision|LineTraceByChannel _worldlocation (+ _worldlocation (* _worlddirection 3e+03)) "TraceTypeQuery1" false 0 "None"))
      (Development|PrintString (Utilities|String|ToString(Vector) (.Location (Collision|BreakHitResult _outhit))))
      (Variables|Default|SetDestination (.Location (Collision|BreakHitResult _outhit))))
    (:then_2
      (Transformation|AddActorWorldOffset (* (Math|Vector|GetUpVector (Transformation|GetActorRotation)) 1.0)))))

(event Input|MouseEvents|LeftMouseButton
  (params (Key :type Key%20Structure :default "None")))

(fn ConstructionScript)