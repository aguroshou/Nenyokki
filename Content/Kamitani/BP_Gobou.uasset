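; BP_Gobou is a Gobou segment actor that swings about the X axis to follow the mouse cursor until it is fixed.
; Each Tick deprojects the cursor to a fixed distance, flattens the direction to the YZ plane, and derives a signed roll from straight down using dot and cross products.
; FixPosition stops the tracking, and GetNextGobouLocation returns the Arrow component's world location as the next Gobou's position.
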(event EventBeginPlay)

(event Collision|EventActorBeginOverlap
  (params (OtherActor :type Actor%20Object%20Reference)))

(event EventTick
  (params (DeltaSeconds :type Float%20%28single-precision%29))
  (bind _returnvalue (* "0, 0,-1.000000" 1.0))
  (if (not (Variables|Default|GetIsFix))
    (bind _returnvalue_2 (Class|WidgetLayoutLibrary|GetMousePositiononViewport))
    (Transformation|SetActorRotation (Math|Rotator|MakeRotator (* (Class|KismetMathLibrary|DegAcos (Math|Vector|DotProduct (Math|Vector|Normalize (* (- (+ (.WorldPosition (Class|GameplayStatics|DeprojectScreentoWorld (Game|GetPlayerController 0) _returnvalue_2)) (* (.WorldDirection (Class|GameplayStatics|DeprojectScreentoWorld (Game|GetPlayerController 0) _returnvalue_2)) 648.065247)) (Transformation|GetActorLocation)) "0,1.000000,1.000000")) _returnvalue)) (Math|Float|Sign(Float) (Math|Vector|DotProduct (Math|Vector|CrossProduct (Math|Vector|Normalize (* (- (+ (.WorldPosition (Class|GameplayStatics|DeprojectScreentoWorld (Game|GetPlayerController 0) _returnvalue_2)) (* (.WorldDirection (Class|GameplayStatics|DeprojectScreentoWorld (Game|GetPlayerController 0) _returnvalue_2)) 648.065247)) (Transformation|GetActorLocation)) "0,1.000000,1.000000")) _returnvalue) "1.000000,0.000000,0.000000"))) 0.0 0.0))))

(fn ConstructionScript)

(fn GetNextGobouLocation
  (return (Transformation|GetWorldLocation (Variables|Default|GetArrow))))

(fn FixPosition
  (Variables|Default|SetIsFix true))