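; Player camera actor that grows a chain of Gobou segments on each left click.
; A click fixes the current Gobou, moves the camera to its next location in X and Z only, spawns a new Gobou there and asks GroundSpawner for more ground.
; FixGobou line-traces along the segment to trigger OnHit on items, applies SpawnCost to the game mode's energy via AddEne and plays the Root sound.
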(event EventBeginPlay)

(event Collision|EventActorBeginOverlap
  (params (OtherActor :type Actor%20Object%20Reference)))

(event EventTick
  (params (DeltaSeconds :type Float%20%28single-precision%29)))

(event Input|MouseEvents|LeftMouseButton
  (params (Key :type Key%20Structure))
  (:Pressed
    (bind _usegobou (Variables|Default|GetUseGobou)
      (:then
        (Default|FixPosition _usegobou)
        (CallFunction|FixGobou)
        (Transformation|SetActorLocation (* (Default|GetNextGobouLocation _usegobou) "1.000000, 0,1.000000") false false)
        (bind _returnvalue (Game|SpawnActorfromClass "/Game/Kamitani/BP_Gobou.BP_Gobou_C" (Math|Transform|MakeTransform (Default|GetNextGobouLocation _usegobou) "0, 0, 0" "1,1,1") "Undefined" 0 0))
        (Variables|Default|SetUseGobou _returnvalue)
        (Default|SpawnGround (Variables|Default|GetGroundSpawner)))
      (:else))))

(fn ConstructionScript)

(fn FixGobou
  (Utilities|FlowControl|Sequence
    (:then_0
      (LocalVariables|SetStart (Transformation|GetActorLocation (Variables|Default|GetUseGobou)))
      (LocalVariables|SetEnd (Default|GetNextGobouLocation (Variables|Default|GetUseGobou)))
      (bind _outhits (Collision|MultiLineTraceByChannel (LocalVariables|GetStart) (LocalVariables|GetEnd) "TraceTypeQuery1" false 0 "None"))
      (for _array_element _outhits
        (bind _asbp_item_base (Utilities|Casting|CastToBP_ItemBase (.HitActor (Collision|BreakHitResult _array_element))))
        (Default|OnHit _asbp_item_base)))
    (:then_1
      (bind _newparam (CallFunction|GetMyGameMode))
      (Default|AddEne _newparam (Variables|Default|GetSpawnCost)))
    (:then_2
      (Audio|SpawnSound2D "/Game/Kamitani/Sound/root.root" 1.0 1.0 0.0 0))))

(fn GetCamra
  (return (Variables|Default|GetCamera)))