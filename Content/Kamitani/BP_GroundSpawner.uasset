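; BP_GroundSpawner is an actor that spawns BP_GroundBord ground pieces along the Z axis based on the player's height.
; SpawnGround compares a spawn counter to the player's Z, offset downward and divided by a spacing value.
; When the counter is behind, it increments and spawns one piece at counter times spacing.
; The event graph is empty, so nothing in this Blueprint calls SpawnGround.
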(event EventBeginPlay)

(event Collision|EventActorBeginOverlap
  (params (OtherActor :type Actor%20Object%20Reference)))

(event EventTick
  (params (DeltaSeconds :type Float%20%28single-precision%29)))

(fn ConstructionScript)

(fn SpawnGround
  (if (< (Variables|Default|GetNewVar_1) (Math|Float|Truncate (/ (+ (.z (Transformation|GetActorLocation (Game|GetPlayerCharacter 0))) -1.8e+03) (LocalVariables|GetNewLocalVar_0))))
    (bind _result (Math|Integer|IncrementInt (Variables|Default|GetNewVar_1))
      (:%20%20
        (Game|SpawnActorfromClass "/Game/Kamitani/BP_GroundBord.BP_GroundBord_C" (Math|Transform|MakeTransform (Math|Vector|MakeVector 0.0 0.0 (* _result (LocalVariables|GetNewLocalVar_0))) "0, 0, 0" "1,1,1") "Undefined" 0 0)))))