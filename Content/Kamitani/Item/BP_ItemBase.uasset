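; BP_ItemBase is a base item actor that awards score and heal value when its OnHit function is called.
; OnHit unhides the Plane component, plays the Item sound in 2D, and adds fixed amounts to Score and HealValue in BP_GameInstance before destroying the actor.
; The event graph holds only disabled stubs, so nothing in this Blueprint calls OnHit itself.
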(event EventBeginPlay)

(event Collision|EventActorBeginOverlap
  (params (OtherActor :type Actor%20Object%20Reference)))

(event EventTick
  (params (DeltaSeconds :type Float%20%28single-precision%29)))

(fn ConstructionScript)

(fn OnHit
  (Development|SetHiddeninGame (Variables|Default|GetPlane) false false)
  (Audio|SpawnSound2D "/Game/Kamitani/Sound/item.item" 1.0 1.0 0.0 0)
  (bind _asbp_game_instance (Utilities|Casting|CastToBP_GameInstance (Game|GetGameInstance)))
  (Variables|/Game/Aguro/BP_GameInstance.BP_GameInstance_C|SetScore _asbp_game_instance (+ (Variables|/Game/Aguro/BP_GameInstance.BP_GameInstance_C|GetScore _asbp_game_instance) 10))
  (Variables|/Game/Aguro/BP_GameInstance.BP_GameInstance_C|SetHealValue _asbp_game_instance (+ (Variables|/Game/Aguro/BP_GameInstance.BP_GameInstance_C|GetHealValue _asbp_game_instance) 50))
  (Actor|DestroyActor))