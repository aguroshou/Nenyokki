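; Game mode that runs a depleting gauge, starting at its maximum, and shows the results screen when it empties through AddEne.
; Tick drains the gauge at a rate that rises every frame, then consumes HealValue from BP_GameInstance and caps the total.
; AddEne applies a change to the gauge and, at zero or below, opens Result_UI with the GameInstance score and calls Rank.
; Tick itself never checks for depletion.
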(event EventBeginPlay
  (Variables|Default|SetGauge (Variables|Default|GetMaxGauge)))

(event EventTick
  (params (DeltaSeconds :type Float%20%28single-precision%29))
  (bind _maxgauge (Variables|Default|GetMaxGauge))
  (Variables|Default|SetGauge (- (Variables|Default|GetGauge) (* DeltaSeconds (Variables|Default|GetGaugeDecreaseRate))))
  (Variables|Default|SetGaugeDecreaseRate (+ (Variables|Default|GetGaugeDecreaseRate) 0.01))
  (bind _asbp_game_instance (Utilities|Casting|CastToBP_GameInstance (Game|GetGameInstance)))
  (Variables|Default|SetGauge (+ (Variables|Default|GetGauge) (Math|Conversions|ToFloat(Integer) (Variables|/Game/Aguro/BP_GameInstance.BP_GameInstance_C|GetHealValue _asbp_game_instance))))
  (Variables|/Game/Aguro/BP_GameInstance.BP_GameInstance_C|SetHealValue _asbp_game_instance 0)
  (if (> (Variables|Default|GetGauge) _maxgauge)
    (Variables|Default|SetGauge _maxgauge)))

(fn ConstructionScript)

(fn AddEne
  (params (NewParam :type Float%20%28single-precision%29))
  (bind _output_get (Variables|Default|SetGauge (Math|Float|Min(Float) (+ NewParam (Variables|Default|GetGauge)) (Variables|Default|GetMaxGauge))))
  (if (<= _output_get 0.0)
    (bind _returnvalue (UserInterface|CreateWidget "/Game/Incl/UI/GameMain/Result_UI.Result_UI_C"))
    (UserInterface|Viewport|AddtoViewport _returnvalue 0)
    (bind _asbp_game_instance (Utilities|Casting|CastToBP_GameInstance (Game|GetGameInstance)))
    (Variables|/Game/Incl/UI/GameMain/Result_UI.Result_UI_C|SetTestInt _returnvalue (Variables|/Game/Aguro/BP_GameInstance.BP_GameInstance_C|GetScore _asbp_game_instance))
    (Default|Rank _returnvalue)))